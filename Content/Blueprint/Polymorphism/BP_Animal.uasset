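; BP_Animal is an animal actor that takes its name, noise text, mesh and material from its TypeOfAnimal enum (Capybara, Bear or Pig).
; The construction script calls one helper per feature, using the enum as an index into noise, mesh and material arrays and its string form as the name.
; The type switch has empty branches, and BeginPlay only writes a trace bookmark, as the construction script also does.
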(event `self.ReceiveBeginPlay`
  (`TraceUtilLibrary.TraceBookmark` "START THE GAME"))

(fn `MaterialAnimal`
  (params (self2 :type "PrimitiveComponent Object Reference") (Value :type Byte))
  (`PrimitiveComponent.SetMaterial` self2 0 (`|GetArrayItem` (`self.AnimalMaterial`) (`KismetMathLibrary.Conv_ByteToInt` (`KismetSystemLibrary.MakeLiteralByte` Value)))))

(fn `NameAnimal`
  (params (Value :type Byte))
  (locals (LocalAnimalName :type String))
  (bind _output_get (set `local.LocalAnimalName` (`|GetEnumeratorNameAsString` (cast `/Game/Blueprint/Polymorphism/E_AnimalType` Value))))
  (`TextRenderComponent.K2_SetText` (`self.AnimalName`) (`KismetTextLibrary.Conv_StringToText` _output_get)))

(fn `NoiseAnimal`
  (params (Value :type Byte))
  (`TextRenderComponent.K2_SetText` (`self.AnimalNoise`) (`|GetArrayItem` (`self.NoiseOfAnimal`) (`KismetMathLibrary.Conv_ByteToInt` (`KismetSystemLibrary.MakeLiteralByte` Value)))))

(fn `StaticMeshAnimal`
  (params (Value :type Byte))
  (returns (ObjectStaticMesh :type "StaticMeshComponent Object Reference"))
  (bind _objectstaticmesh (`self.ObjectStaticMesh`))
  (`StaticMeshComponent.SetStaticMesh` _objectstaticmesh (`|GetArrayItem` (`self.StaticMesh`) (`KismetMathLibrary.Conv_ByteToInt` (`KismetSystemLibrary.MakeLiteralByte` Value))))
  (return _objectstaticmesh))

(fn `UserConstructionScript`
  (bind _typeofanimal (`self.TypeOfAnimal`))
  (`TraceUtilLibrary.TraceBookmark` "BUILD THE ANIMAL")
  (switch `/Game/Blueprint/Polymorphism/E_AnimalType` _typeofanimal
    (:`NewEnumerator0`
      _)
    (:`NewEnumerator1`
      _)
    (:`NewEnumerator2`
      _))
  (`self.NameAnimal` _typeofanimal)
  (`self.NoiseAnimal` _typeofanimal)
  (bind _objectstaticmesh (`self.StaticMeshAnimal` _typeofanimal))
  (`self.MaterialAnimal` _objectstaticmesh _typeofanimal))