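; BP_Toy is a toy pickup actor configured from a ToyStructure enum and its parallel arrays.
; The construction script uses the enum as an index to set name and noise texts, mesh, material and happiness value.
; On box overlap it sends PickUpTwoHandsMessage with happiness and DoToysData's mesh and material outputs to the other actor, then destroys itself without filtering who overlapped.
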(event `self.Box.OnComponentBeginOverlap`
  (params (OverlappedComponent :type "PrimitiveComponent Object Reference") (OtherActor :type "Actor Object Reference") (OtherComp :type "PrimitiveComponent Object Reference") (OtherBodyIndex :type Integer) (bFromSweep :type Boolean) (SweepResult :type "HitResult Structure (by ref)"))
  (bind (_toyenum _toynoise _toystaticmesh _toymaterial) (break `/Game/Blueprint/Liskov/F_ToyStruct` (`self.ToyStructure`)))
  (bind _returnvalue (`KismetSystemLibrary.MakeLiteralByte` _toyenum))
  (message `/Game/Blueprint/Liskov/ISP/BPI_PickUpObject.PickUpTwoHands` OtherActor (`self.ToyHappiness`) (`|GetArrayItem` _toystaticmesh (`KismetMathLibrary.Conv_ByteToInt` _returnvalue)) (`|GetArrayItem` _toymaterial (`KismetMathLibrary.Conv_ByteToInt` _returnvalue)))
  (`self.K2_DestroyActor`))

(fn `HappinessfromToy`
  (params (Value :type Byte) (Array :type "Array of Integer"))
  (set `self.ToyHappiness` (`|GetArrayItem` Array (`KismetMathLibrary.Conv_ByteToInt` (`KismetSystemLibrary.MakeLiteralByte` Value)))))

(fn `MaterialToy`
  (params (self2 :type "PrimitiveComponent Object Reference") (Value :type Byte) (Array :type "Array of Material Object Reference"))
  (`PrimitiveComponent.SetMaterial` self2 0 (`|GetArrayItem` Array (`KismetMathLibrary.Conv_ByteToInt` (`KismetSystemLibrary.MakeLiteralByte` Value)))))

(fn `NameToy`
  (params (Enumerator :type "/Game/Blueprint/Liskov/E_ToyTypes Enum" :default "NewEnumerator0"))
  (`TextRenderComponent.K2_SetText` (`self.ToyName`) (`KismetTextLibrary.Conv_StringToText` (`|GetEnumeratorNameAsString` Enumerator))))

(fn `NoiseToy`
  (params (Value :type Byte) (Array :type "Array of Text"))
  (`TextRenderComponent.K2_SetText` (`self.ToyNoise`) (`|GetArrayItem` Array (`KismetMathLibrary.Conv_ByteToInt` (`KismetSystemLibrary.MakeLiteralByte` Value)))))

(fn `StaticMeshToy`
  (params (Value :type Byte) (Array :type "Array of StaticMesh Object Reference"))
  (returns (ToyMesh :type "StaticMeshComponent Object Reference"))
  (bind _toymesh (`self.ToyMesh`))
  (`StaticMeshComponent.SetStaticMesh` _toymesh (`|GetArrayItem` Array (`KismetMathLibrary.Conv_ByteToInt` (`KismetSystemLibrary.MakeLiteralByte` Value))))
  (return _toymesh))

(fn `UserConstructionScript`
  (bind (_toyenum _toynoise _toystaticmesh _toymaterial _happiness) (break `/Game/Blueprint/Liskov/F_ToyStruct` (`self.ToyStructure`)))
  (switch `/Game/Blueprint/Liskov/E_ToyTypes` _toyenum
    (:`NewEnumerator0`
      (`self.NameToy` _toyenum)
      (`self.NoiseToy` _toyenum _toynoise)
      (bind _toymesh (`self.StaticMeshToy` _toyenum _toystaticmesh))
      (`self.MaterialToy` _toymesh _toyenum _toymaterial)
      (`self.HappinessfromToy` _toyenum _happiness))))